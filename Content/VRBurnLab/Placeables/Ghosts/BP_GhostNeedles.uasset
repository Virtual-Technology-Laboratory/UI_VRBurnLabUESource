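; Ghost placeholder for the needles in the VR burn lab, filled when a tagged object hits it.
; On Hit, if the other actor's root component has the tag and is simulating physics, that actor is destroyed.
; The ghost applies solid materials, destroys itself, reveals the referenced needle group and sets the Needles flag on GM_LabVR.
; A Filled flag guards against repeat fills.
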(event `self.ReceiveHit`
  (params (MyComp :type "PrimitiveComponent Object Reference") (Other :type "Actor Object Reference") (OtherComp :type "PrimitiveComponent Object Reference") (bSelfMoved :type Boolean) (HitLocation :type "Vector Structure") (HitNormal :type "Vector Structure") (NormalImpulse :type "Vector Structure") (Hit :type "HitResult Structure (by ref)"))
  (bind _rootcomponent (`Actor.RootComponent` Other))
  (if (`self.Filled`)
    _
    (elif (`ActorComponent.ComponentHasTag` _rootcomponent (`self.Tag`))
      (if (`SceneComponent.IsAnySimulatingPhysics` _rootcomponent)
        (`self.K2_DestroyActor` Other)
        (`PrimitiveComponent.SetMaterial` (`self.StaticMesh`) 0 "/Game/Geometry/Meshes/CubeMaterial.CubeMaterial")
        (`PrimitiveComponent.SetMaterial` (`self.Needles2`) 0 "/Game/VRBurnLab/MaterialLibrary/BurnLabObjects/M_Needles.M_Needles")
        (`PrimitiveComponent.SetMaterial` (`self.Needles3`) 0 "/Game/VRBurnLab/MaterialLibrary/BurnLabObjects/M_Needles.M_Needles")
        (`PrimitiveComponent.SetMaterial` (`self.Needles`) 0 "/Game/VRBurnLab/MaterialLibrary/BurnLabObjects/M_Needles.M_Needles")
        (`PrimitiveComponent.SetMaterial` (`self.Needles1`) 0 "/Game/VRBurnLab/MaterialLibrary/BurnLabObjects/M_Needles.M_Needles")
        (set `self.Filled` true)
        (`self.K2_DestroyActor`)
        (`self.SetActorHiddenInGame` (`self.BP_NeedleGroup_Ref`) false)
        (bind _asgm_lab_vr (cast `/Game/VRBurnLab/Core/GM_LabVR` (`GameplayStatics.GetGameMode`)))
        (set `/Game/VRBurnLab/Core/GM_LabVR.Needles` true _asgm_lab_vr)))))

(fn `UserConstructionScript`)