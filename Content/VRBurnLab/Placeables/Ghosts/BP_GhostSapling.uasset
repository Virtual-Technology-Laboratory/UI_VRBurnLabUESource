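; BP_GhostSapling is a ghost placement target for a pine sapling in the VR burn lab.
; When hit by a physics-simulating actor with the matching root-component tag, it destroys that actor and spawns a collisionless BP_PUPineSapling at its own transform.
; It then sets the Sapling flag on GM_LabVR and destroys itself.
; An unconnected chain that would instead swap the ghost's materials to solid ones never runs.
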(event `self.ReceiveHit`
  (params (MyComp :type "PrimitiveComponent Object Reference") (Other :type "Actor Object Reference") (OtherComp :type "PrimitiveComponent Object Reference") (bSelfMoved :type Boolean) (HitLocation :type "Vector Structure") (HitNormal :type "Vector Structure") (NormalImpulse :type "Vector Structure") (Hit :type "HitResult Structure (by ref)"))
  (bind _rootcomponent (`Actor.RootComponent` Other))
  (if (`self.Filled`)
    _
    (elif (`ActorComponent.ComponentHasTag` _rootcomponent (`self.Tag`))
      (if (`SceneComponent.IsAnySimulatingPhysics` _rootcomponent)
        (`self.K2_DestroyActor` Other)
        (bind _returnvalue (`|SpawnActorFromClass` "/Game/VRBurnLab/Placeables/Pickups/BP_PUPineSapling.BP_PUPineSapling_C" (`self.GetTransform`) "AlwaysSpawn" "OverrideRootScale" null null))
        (`PrimitiveComponent.SetCollisionEnabled` (`StaticMeshActor.StaticMeshComponent` _returnvalue) "NoCollision")
        (set `self.Filled` true)
        (bind _asgm_lab_vr (cast `/Game/VRBurnLab/Core/GM_LabVR` (`GameplayStatics.GetGameMode`)))
        (set `/Game/VRBurnLab/Core/GM_LabVR.Sapling` true _asgm_lab_vr)
        (`self.K2_DestroyActor`)))))

(fn `UserConstructionScript`)