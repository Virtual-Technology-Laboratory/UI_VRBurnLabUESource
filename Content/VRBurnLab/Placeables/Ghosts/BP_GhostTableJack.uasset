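; Ghost placeholder for a table jack in the VR burn lab that the player fills by bringing a matching object into it.
; On Hit, if still unfilled, it checks the other actor's root component for a tag and simulated physics, then destroys that actor.
; It then swaps both material slots to solid materials, marks itself filled and increments the Jacks count on GM_LabVR.
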(event `self.ReceiveHit`
  (params (MyComp :type "PrimitiveComponent Object Reference") (Other :type "Actor Object Reference") (OtherComp :type "PrimitiveComponent Object Reference") (bSelfMoved :type Boolean) (HitLocation :type "Vector Structure") (HitNormal :type "Vector Structure") (NormalImpulse :type "Vector Structure") (Hit :type "HitResult Structure (by ref)"))
  (bind _rootcomponent (`Actor.RootComponent` Other))
  (bind _staticmeshcomponent (`self.StaticMeshComponent`))
  (if (`self.Filled`)
    _
    (elif (`ActorComponent.ComponentHasTag` _rootcomponent (`self.Tag`))
      (if (`SceneComponent.IsAnySimulatingPhysics` _rootcomponent)
        (`self.K2_DestroyActor` Other)
        (`|ExecutionSequence`
          (:`then_0`
            (`PrimitiveComponent.SetMaterial` _staticmeshcomponent 0 (`self.Material`)))
          (:`then_1`
            (`PrimitiveComponent.SetMaterial` _staticmeshcomponent 1 "/Game/VRBurnLab/Placeables/Pickups/M_JackPlastic.M_JackPlastic")
            (set `self.Filled` true)
            (bind _asgm_lab_vr (cast `/Game/VRBurnLab/Core/GM_LabVR` (`GameplayStatics.GetGameMode`)))
            (bind _jacks (`/Game/VRBurnLab/Core/GM_LabVR.Jacks` _asgm_lab_vr))
            (`/Engine/EditorBlueprintResources/StandardMacros.IncrementInt` _jacks
              (:`  `
                (set `/Game/VRBurnLab/Core/GM_LabVR.Jacks` _jacks _asgm_lab_vr)))))))))

(fn `UserConstructionScript`)