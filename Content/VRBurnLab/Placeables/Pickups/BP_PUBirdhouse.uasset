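; VR pickup birdhouse that can be wrapped in foil or soaked with water taken from foil box and water bottle references.
; Overlap previews the metal or wet-board material and foil planes while a source holds that resource, reverting on exit unless applied.
; RayInteract during overlap commits the change and clears the sources' flags.
; Pickup and Drop toggle physics and attachment, while custom depth stencil highlights the unheld birdhouse on overlap.
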(event `self.Overlap_01.OnComponentBeginOverlap`
  (params (OverlappedComponent :type "PrimitiveComponent Object Reference") (OtherActor :type "Actor Object Reference") (OtherComp :type "PrimitiveComponent Object Reference") (OtherBodyIndex :type Integer) (bFromSweep :type Boolean) (SweepResult :type "HitResult Structure (by ref)"))
  (bind _staticmesh (`self.StaticMesh`))
  (bind _staticmesh_2 (`self.StaticMesh`))
  ;[1 1 1] Detect overlap
  (`|ExecutionSequence`
    (:`then_0`
      (for _array_element (`self.BP_FoilBox_Ref`)
        (if (`/Game/VRBurnLab/Placeables/Interactions/BP_FoilBox.HasFoil?` _array_element)
          (`PrimitiveComponent.SetMaterial` _staticmesh 1 "/Game/VRBurnLab/MaterialLibrary/M_GenericMetal.M_GenericMetal")
          (set `self.IsOverlap_01` true)
          (`SceneComponent.SetVisibility` (`self.Plane`) true false)
          (`SceneComponent.SetVisibility` (`self.Plane3`) true false)
          (`SceneComponent.SetVisibility` (`self.Plane2`) true false)
          (`SceneComponent.SetVisibility` (`self.Plane4`) true false)
          (`SceneComponent.SetVisibility` (`self.Plane5`) true false)
          (`SceneComponent.SetVisibility` (`self.Plane6`) true false)
          (`SceneComponent.SetVisibility` (`self.Plane1`) true false))))
    (:`then_1`
      (for _array_element_2 (`self.WaterBottleRef`)
        (if (`/Game/VRBurnLab/Placeables/Interactions/BP_WaterBottle.HasWater?` _array_element_2)
          (`PrimitiveComponent.SetMaterial` _staticmesh 0 "/Game/VRBurnLab/Placeables/Pickups/M_WetBoard.M_WetBoard")
          (set `self.IsOverlap_01` true))))
    (:`then_2`
      (if (not (`self.IsPickedUp?`))
        (`PrimitiveComponent.SetRenderCustomDepth` _staticmesh_2 true)
        (`PrimitiveComponent.SetCustomDepthStencilValue` _staticmesh_2 2)))))

(event `self.Overlap_01.OnComponentEndOverlap`
  (params (OverlappedComponent :type "PrimitiveComponent Object Reference") (OtherActor :type "Actor Object Reference") (OtherComp :type "PrimitiveComponent Object Reference") (OtherBodyIndex :type Integer))
  (bind _staticmesh (`self.StaticMesh`))
  (bind _staticmesh_2 (`self.StaticMesh`))
  ;[1 1 1] Detect overlap
  (`|ExecutionSequence`
    (:`then_0`
      (if (not (`self.HasFoil?`))
        (`PrimitiveComponent.SetMaterial` _staticmesh 1 "/Game/VRBurnLab/Placeables/Pickups/M_Board.M_Board")
        (set `self.IsOverlap_01` false)
        (`SceneComponent.SetVisibility` (`self.Plane`) false false)
        (`SceneComponent.SetVisibility` (`self.Plane3`) false false)
        (`SceneComponent.SetVisibility` (`self.Plane2`) false false)
        (`SceneComponent.SetVisibility` (`self.Plane4`) false false)
        (`SceneComponent.SetVisibility` (`self.Plane5`) false false)
        (`SceneComponent.SetVisibility` (`self.Plane6`) false false)
        (`SceneComponent.SetVisibility` (`self.Plane1`) false false)))
    (:`then_1`
      (if (not (`self.HasWater?`))
        (`PrimitiveComponent.SetMaterial` _staticmesh 0 "/Game/VRBurnLab/Placeables/Pickups/M_Board.M_Board")
        (set `self.IsOverlap_01` false)))
    (:`then_2`
      (`PrimitiveComponent.SetRenderCustomDepth` _staticmesh_2 false)
      (`PrimitiveComponent.SetCustomDepthStencilValue` _staticmesh_2 0))))

(event `/Game/VRBurnLab/Core/Character/RayActorInterface.RayInteract`
  ;[1 1 1] Switch materials when interacted with
  (`|ExecutionSequence`
    (:`then_0`
      (for _array_element (`self.BP_FoilBox_Ref`)
        (if (`/Game/VRBurnLab/Placeables/Interactions/BP_FoilBox.HasFoil?` _array_element)
          (if (`self.IsOverlap_01`)
            (`PrimitiveComponent.SetMaterial` (`self.StaticMesh`) 1 "/Game/VRBurnLab/MaterialLibrary/M_GenericMetal.M_GenericMetal")
            (set `self.HasFoil?` true)
            (for _array_element_2 (`self.BP_FoilBox_Ref`)
              (set `/Game/VRBurnLab/Placeables/Interactions/BP_FoilBox.HasFoil?` false _array_element_2)
              (`SceneComponent.SetVisibility` (`self.Plane`) true false)
              (`SceneComponent.SetVisibility` (`self.Plane3`) true false)
              (`SceneComponent.SetVisibility` (`self.Plane2`) true false)
              (`SceneComponent.SetVisibility` (`self.Plane4`) true false)
              (`SceneComponent.SetVisibility` (`self.Plane5`) true false)
              (`SceneComponent.SetVisibility` (`self.Plane6`) true false)
              (`SceneComponent.SetVisibility` (`self.Plane1`) true false))))))
    (:`then_1`
      (if (`self.IsOverlap_01`)
        (for _array_element_3 (`self.WaterBottleRef`)
          (if (`/Game/VRBurnLab/Placeables/Interactions/BP_WaterBottle.HasWater?` _array_element_3)
            (`PrimitiveComponent.SetMaterial` (`self.StaticMesh`) 0 "/Game/VRBurnLab/Placeables/Pickups/M_WetBoard.M_WetBoard")
            (set `self.HasWater?` true)
            (for _array_element_4 (`self.WaterBottleRef`)
              (set `/Game/VRBurnLab/Placeables/Interactions/BP_WaterBottle.HasWater?` false _array_element_4))))))))

(event `/Game/VirtualRealityBP/Blueprints/PickupActorInterface.Pickup`
  (params (AttachTo :type "SceneComponent Object Reference"))
  (bind _staticmesh (`self.StaticMesh`))
  (set `self.IsPickedUp?` true)
  (`PrimitiveComponent.SetSimulatePhysics` (`self.StaticMesh`) false)
  (`SceneComponent.K2_AttachToComponent` (`self.K2_GetRootComponent`) AttachTo "None" "KeepWorld" "KeepWorld" "KeepWorld" false)
  (`PrimitiveComponent.SetRenderCustomDepth` _staticmesh false)
  (`PrimitiveComponent.SetCustomDepthStencilValue` _staticmesh 0))

(event `/Game/VirtualRealityBP/Blueprints/PickupActorInterface.Drop`
  (set `self.IsPickedUp?` false)
  (`PrimitiveComponent.SetSimulatePhysics` (`self.StaticMesh`) true)
  (`self.K2_DetachFromActor` "KeepWorld" "KeepWorld" "KeepWorld"))

(fn `UserConstructionScript`)