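; BP_Screen_2 is a video screen placeable in the VR burn lab that plays recorded fuel burn clips.
; Four custom events each open a different media source on its MediaPlayer: normal fuel with or without foil, and heavy fuel with or without water.
; The events only switch the source, with no other playback logic and an empty construction script.
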(event `NormalFuel2`
  (`MediaPlayer.OpenSource` (`self.MediaPlayer`) "/Game/Movies/NFuel_NoFoil.NFuel_NoFoil"))

(event `NFuel_Foil2`
  (`MediaPlayer.OpenSource` (`self.MediaPlayer`) "/Game/Movies/NFuel.NFuel"))

(event `HeavyFuel2`
  (`MediaPlayer.OpenSource` (`self.MediaPlayer`) "/Game/Movies/HFuel.HFuel"))

(event `HFuel_Water2`
  (`MediaPlayer.OpenSource` (`self.MediaPlayer`) "/Game/Movies/HFuel_Water.HFuel_Water"))

(fn `UserConstructionScript`)