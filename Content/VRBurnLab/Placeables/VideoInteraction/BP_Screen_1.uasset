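; BP_Screen_1 is an in-world screen for the VR burn lab that plays camera footage of fuel burn experiments.
; Four custom events (normal fuel, normal fuel with foil, heavy fuel, heavy fuel with water) each open their matching media source on a MediaPlayer.
; It holds no other logic, so whatever calls these events selects the clip.
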(event `NormalFuel`
  (`MediaPlayer.OpenSource` (`self.MediaPlayer`) "/Game/Movies/BLCam_NFuel_NoFoil.BLCam_NFuel_NoFoil"))

(event `NFuel_Foil`
  (`MediaPlayer.OpenSource` (`self.MediaPlayer`) "/Game/Movies/BLCam_NFuel.BLCam_NFuel"))

(event `HeavyFuel`
  (`MediaPlayer.OpenSource` (`self.MediaPlayer`) "/Game/Movies/BLCam_HFuel.BLCam_HFuel"))

(event `HFuel_Water`
  (`MediaPlayer.OpenSource` (`self.MediaPlayer`) "/Game/Movies/BLCam_HFuel_Water.BLCam_HFuel_Water"))

(fn `UserConstructionScript`)