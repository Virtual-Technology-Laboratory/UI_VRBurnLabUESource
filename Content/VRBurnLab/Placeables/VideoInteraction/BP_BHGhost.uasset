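; BP_BHGhost is a ghost placement target for pickup birdhouses in VR Burn Lab.
; On a hit by a tagged actor while not Filled, it finds the matching birdhouse in PUBirdhouseRef by object name and copies its foil and water flags.
; If that actor is simulating physics, it moves the birdhouse mesh to the ghost's transform and hides its own mesh.
; Filled is only read here, never set.
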(event `self.ReceiveHit`
  (params (MyComp :type "PrimitiveComponent Object Reference") (Other :type "Actor Object Reference") (OtherComp :type "PrimitiveComponent Object Reference") (bSelfMoved :type Boolean) (HitLocation :type "Vector Structure") (HitNormal :type "Vector Structure") (NormalImpulse :type "Vector Structure") (Hit :type "HitResult Structure (by ref)"))
  (bind _rootcomponent (`Actor.RootComponent` Other))
  (if (`self.Filled`)
    _
    (elif (`ActorComponent.ComponentHasTag` _rootcomponent (`self.Tag`))
      ;[1 1 1] Get specific array element has foil bool
      (for _array_element (`self.PUBirdhouseRef`)
        (if (`KismetStringLibrary.EqualEqual_StrStr` (`KismetSystemLibrary.GetObjectName` Other) (`KismetSystemLibrary.GetObjectName` _array_element))
          (if (`/Game/VRBurnLab/Placeables/Pickups/BP_PUBirdhouse.HasFoil?` _array_element)
            (set `self.HasFoil?` true)
            (else
              (set `self.HasFoil?` false)))
          ;[1 1 1] Get specific array element has water bool
          (for _array_element_2 (`self.PUBirdhouseRef`)
            (if (`KismetStringLibrary.EqualEqual_StrStr` (`KismetSystemLibrary.GetObjectName` Other) (`KismetSystemLibrary.GetObjectName` _array_element_2))
              (if (`/Game/VRBurnLab/Placeables/Pickups/BP_PUBirdhouse.HasWater?` _array_element_2)
                (set `self.HasWater?` true)
                (else
                  (set `self.HasWater?` false)))
              (if (`SceneComponent.IsAnySimulatingPhysics` _rootcomponent)
                (for _array_element_3 (`self.PUBirdhouseRef`)
                  (if (`KismetStringLibrary.EqualEqual_StrStr` (`KismetSystemLibrary.GetObjectName` Other) (`KismetSystemLibrary.GetObjectName` _array_element_3))
                    (`SceneComponent.K2_SetRelativeTransform` (`/Game/VRBurnLab/Placeables/Pickups/BP_PUBirdhouse.StaticMesh` _array_element_3) (`self.GetTransform`) false false)
                    (`SceneComponent.SetVisibility` (`self.StaticMesh`) false false)))))))))))

(fn `UserConstructionScript`)