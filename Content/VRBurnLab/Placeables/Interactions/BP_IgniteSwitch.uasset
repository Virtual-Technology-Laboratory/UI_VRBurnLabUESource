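; BP_IgniteSwitch is a VR burn lab switch that highlights through custom depth stencil on overlap and toggles on Pickup.
; A FlipFlop drives On/Off timelines that rotate the mesh, play or pause two media players and show or hide screen actors.
; Switching on starts Niagara fire and delayed looped-back audio only if GM_LabVR's Needles is set; switching off stops both.
; A delayed DoOnce reset debounces presses, each with a click sound.
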(event `self.StaticMesh.OnComponentBeginOverlap`
  (params (OverlappedComponent :type "PrimitiveComponent Object Reference") (OtherActor :type "Actor Object Reference") (OtherComp :type "PrimitiveComponent Object Reference") (OtherBodyIndex :type Integer) (bFromSweep :type Boolean) (SweepResult :type "HitResult Structure (by ref)"))
  (bind _staticmesh (`self.StaticMesh`))
  (`PrimitiveComponent.SetRenderCustomDepth` _staticmesh true)
  (`PrimitiveComponent.SetCustomDepthStencilValue` _staticmesh 2))

(event `self.StaticMesh.OnComponentEndOverlap`
  (params (OverlappedComponent :type "PrimitiveComponent Object Reference") (OtherActor :type "Actor Object Reference") (OtherComp :type "PrimitiveComponent Object Reference") (OtherBodyIndex :type Integer))
  (bind _staticmesh (`self.StaticMesh`))
  (`PrimitiveComponent.SetRenderCustomDepth` _staticmesh false)
  (`PrimitiveComponent.SetCustomDepthStencilValue` _staticmesh 0))

(event `/Game/VirtualRealityBP/Blueprints/PickupActorInterface.Pickup`
  (params (AttachTo :type "SceneComponent Object Reference"))
  (bind _staticmesh (`self.StaticMesh`))
  (bind _sound (`self.Sound`))
  (`/Engine/EditorBlueprintResources/StandardMacros.DoOnce` false :!label _label
    (:`Completed`
      (`|ExecutionSequence`
        (:`then_0`
          (`/Engine/EditorBlueprintResources/StandardMacros.FlipFlop`
            (:`A`
              (`Timeline|On`
                (:`Update`
                  (`SceneComponent.K2_SetRelativeRotation` _staticmesh (struct :`Roll` 180.0) false false)
                  (`|ExecutionSequence`
                    (:`then_0`
                      (`MediaPlayer.Play` (`self.MediaPlayer`))
                      (`MediaPlayer.Play` (`self.MediaPlayer2`))
                      (`|ExecutionSequence`
                        (:`then_0`
                          (for _array_element (`self.Screen2Ref`)
                            (`SceneComponent.SetVisibility` (`StaticMeshActor.StaticMeshComponent` _array_element) true false :!label _label_2)
                            (`SceneComponent.SetVisibility` (`/Game/VRBurnLab/Placeables/VideoInteraction/BP_Screen_2.Cube` _array_element) true false)
                            (`SceneComponent.SetVisibility` (`StaticMeshActor.StaticMeshComponent` (stale _array_element_2)) true false)
                            (`SceneComponent.SetVisibility` (`/Game/VRBurnLab/Placeables/VideoInteraction/BP_Screen_1.Cube` (stale _array_element_2)) true false)))
                        (:`then_1`
                          (for _array_element_2 (`self.Screen1Ref`)
                            (goto _label_2)))))
                    (:`then_1`
                      (bind _asgm_lab_vr (cast `/Game/VRBurnLab/Core/GM_LabVR` (`GameplayStatics.GetGameMode`)))
                      (if (`/Game/VRBurnLab/Core/GM_LabVR.Needles` _asgm_lab_vr)
                        (`ActorComponent.Activate` (`NiagaraActor.NiagaraComponent` (`self.NS_Fire`)) false)
                        (`KismetSystemLibrary.Delay` 0.2)
                        (`AudioComponent.Play` _sound 0.0)))))))
            (:`B`
              (`Timeline|Off`
                (:`Update`
                  (`SceneComponent.K2_SetRelativeRotation` _staticmesh (struct :`Roll` 225.0) false false)
                  (`MediaPlayer.Pause` (`self.MediaPlayer`))
                  (`MediaPlayer.Pause` (`self.MediaPlayer2`))
                  (for _array_element_3 (`self.Screen1Ref`)
                    (`|ExecutionSequence`
                      (:`then_0`
                        (`SceneComponent.SetVisibility` (`StaticMeshActor.StaticMeshComponent` (stale _array_element_4)) false false :!label _label_3)
                        (`SceneComponent.SetVisibility` (`/Game/VRBurnLab/Placeables/VideoInteraction/BP_Screen_2.Cube` (stale _array_element_4)) false false)
                        (`SceneComponent.SetVisibility` (`StaticMeshActor.StaticMeshComponent` _array_element_3) false false)
                        (`SceneComponent.SetVisibility` (`/Game/VRBurnLab/Placeables/VideoInteraction/BP_Screen_1.Cube` _array_element_3) false false)
                        (`ActorComponent.Deactivate` (`NiagaraActor.NiagaraComponent` (`self.NS_Fire`)))
                        (`KismetSystemLibrary.Delay` 0.2)
                        (`AudioComponent.Stop` _sound))
                      (:`then_1`
                        (for _array_element_4 (`self.Screen2Ref`)
                          (goto _label_3))))))))))
        (:`then_1`
          (`GameplayStatics.PlaySoundAtLocation` "/Game/VRBurnLab/Core/Menu/Click.Click" (`self.K2_GetActorLocation`) (struct) 1.0 1.0 0.0 null null null))
        (:`then_2`
          (`KismetSystemLibrary.Delay` 0.6)
          (goto _label :!via `Reset`))))))

(event `self.ReceiveBeginPlay`
  (bind _returnvalue (`GameplayStatics.SpawnSound2D` "/Game/VRBurnLab/Effects/Fire/fire.fire" 1.0 1.0 0.0 null false false))
  (bind _output_get (set `self.Sound` _returnvalue))
  (`ActorComponent.SetActive` _output_get false false))

(fn `UserConstructionScript`)