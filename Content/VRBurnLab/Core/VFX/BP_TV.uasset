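; BP_TV is an interactive TV in VRBurnLab that toggles its screen between a "Live Action" burn video and a "Simulation" material.
; Actor overlap recolours the label and shows or hides the VR right controller's pointer, skipped when testing with the FPS pawn.
; RayInteract flip-flops the screen material and label, opening and playing the media source if not already playing.
; A DoOnce with delayed reset debounces the toggle.
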(event `self.ReceiveBeginPlay`
  (bind _output_get (set `self.Testing` (`KismetStringLibrary.EqualEqual_StrStr` (`KismetSystemLibrary.GetObjectName` (`GameplayStatics.GetPlayerPawn` 0)) "BP_FPS_C_0")))
  (if (not _output_get)
    (bind _outactors (`GameplayStatics.GetAllActorsOfClass` "/Game/VirtualRealityBP/Blueprints/MotionControllerPawn.MotionControllerPawn_C"))
    (set `self.Right Controller` (`/Game/VirtualRealityBP/Blueprints/MotionControllerPawn.RightController` (`|GetArrayItem` _outactors)))))

(event `self.ReceiveActorBeginOverlap`
  (params (OtherActor :type "Actor Object Reference"))
  (bind _right_controller (`self.Right Controller`))
  (bind _pointer (`/Game/VirtualRealityBP/Blueprints/BP_MotionController.pointer` _right_controller))
  (`TextRenderComponent.SetTextRenderColor` (`self.text`) (`KismetMathLibrary.Conv_LinearColorToColor` (`KismetMathLibrary.MakeColor` 0.0 0.0 1.0)))
  (if (not (`self.Testing`))
    (set `self.IsOverlaped` (== OtherActor _right_controller))
    (`SceneComponent.SetVisibility` _pointer true false)
    (`SceneComponent.SetVisibility` (`/Game/VirtualRealityBP/Blueprints/BP_MotionController.pointer_ball` _right_controller) true false)
    (`SceneComponent.K2_SetRelativeLocation` _pointer (319.0 0.0 0.0) false false)
    (`SceneComponent.K2_SetRelativeLocation` (`/Game/VirtualRealityBP/Blueprints/BP_MotionController.pointer_ball` _right_controller) (319.0 0.0 0.0) false false)))

(event `self.ReceiveActorEndOverlap`
  (params (OtherActor :type "Actor Object Reference"))
  (bind _pointer (`/Game/VirtualRealityBP/Blueprints/BP_MotionController.pointer` (`self.Right Controller`)))
  (set `self.IsOverlaped` false)
  (`TextRenderComponent.SetTextRenderColor` (`self.text`) (`KismetMathLibrary.Conv_LinearColorToColor` (`KismetMathLibrary.MakeColor` 0.0)))
  (if (not (`self.Testing`))
    (`SceneComponent.SetVisibility` _pointer false false)
    (`SceneComponent.SetVisibility` (`/Game/VirtualRealityBP/Blueprints/BP_MotionController.pointer_ball` (`self.Right Controller`)) false false)
    (`SceneComponent.K2_SetRelativeLocation` _pointer (319.0 -100.0 0.0) false false)
    (`SceneComponent.K2_SetRelativeLocation` (`/Game/VirtualRealityBP/Blueprints/BP_MotionController.pointer_ball` (`self.Right Controller`)) (319.0 -100.0 0.0) false false)))

(event `/Game/VRBurnLab/Core/Character/RayActorInterface.RayInteract`
  (bind _mediaplayer (`self.MediaPlayer`))
  (`|DoOnceMultiInput` :!label _label
    (:`A Out`
      (`/Engine/EditorBlueprintResources/StandardMacros.FlipFlop`
        (:`A`
          (`PrimitiveComponent.SetMaterial` (`self.StaticMeshComponent`) 1 "/Game/VRBurnLab/Core/VFX/M_BurnVideo.M_BurnVideo")
          (`TextRenderComponent.K2_SetText` (`self.text`) (`KismetTextLibrary.Conv_StringToText` "Live Action"))
          (if (not (`MediaPlayer.IsPlaying` (`self.MediaPlayer`)))
            (bind _returnvalue (`MediaPlayer.OpenSource` _mediaplayer "/Game/VRBurnLab/Core/VFX/MS_BurnVideo.MS_BurnVideo"))
            (`KismetSystemLibrary.Delay` 0.05 :!label _label_2)
            (if _returnvalue
              (`MediaPlayer.Play` _mediaplayer)
              (else
                (goto _label_2)))))
        (:`B`
          (`PrimitiveComponent.SetMaterial` (`self.StaticMeshComponent`) 1 "/Game/VRBurnLab/Core/VFX/M_Screen.M_Screen")
          (`TextRenderComponent.K2_SetText` (`self.text`) (`KismetTextLibrary.Conv_StringToText` "Simulation"))))
      (`KismetSystemLibrary.Delay` 0.5)
      (goto _label :!via `Reset In`))))

(fn `UserConstructionScript`)