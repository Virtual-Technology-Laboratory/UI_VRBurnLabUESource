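; BP_FPS is a first-person player character with look and move input, ray interaction and object pickup.
; Pressing Fire traces from the camera against WorldDynamic objects and sends RayInteractMessage to the hit actor.
; It also scans the Sphere's overlaps for PickupActorInterface actors, sending PickupMessage whenever one is nearer than the best so far.
; Releasing Fire or pressing Fire2 drops the grabbed actor and resets the distance tracker.
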(event `InputAxis|LookVertical`
  (params (AxisValue :type "Float (single-precision)"))
  ;[1 1 1] Rotation
  (`self.AddControllerPitchInput` AxisValue))

(event `InputAxis|MoveForward`
  (params (AxisValue :type "Float (single-precision)"))
  ;[1 1 1] Movement
  (`self.AddMovementInput` (`KismetMathLibrary.GetForwardVector` (`self.GetControlRotation`)) AxisValue))

(event `InputAxis|LookHorizontal`
  (params (AxisValue :type "Float (single-precision)"))
  ;[1 1 1] Rotation
  (`self.AddControllerYawInput` AxisValue))

(event `InputAxis|MoveRight`
  (params (AxisValue :type "Float (single-precision)"))
  ;[1 1 1] Movement
  (`self.AddMovementInput` (`KismetMathLibrary.GetRightVector` (`self.GetControlRotation`)) AxisValue))

(event `InputAction|Fire2`
  (params (Key :type "Key Structure"))
  (:`Pressed`
    (message `/Game/VirtualRealityBP/Blueprints/PickupActorInterface.Drop` (`self.GrabbedActor`) :!label _label)
    (set `self.GrabbedActor` null)
    (set `self.NearestOverlap` 10000.0)))

(event `InputAction|Fire`
  (params (Key :type "Key Structure"))
  (bind _sphere (`self.Sphere`))
  (:`Pressed`
    (`self.FireRay`)
    (for _array_element (`PrimitiveComponent.GetOverlappingActors` _sphere "/Script/Engine.Actor")
      (if (`KismetSystemLibrary.DoesImplementInterface` _array_element "/Game/VirtualRealityBP/Blueprints/PickupActorInterface.PickupActorInterface_C")
        (bind _returnvalue (`KismetMathLibrary.VSize` (- (`self.K2_GetActorLocation` _array_element) (`SceneComponent.K2_GetComponentLocation` _sphere))))
        (if (< _returnvalue (`self.NearestOverlap`))
          (bind _output_get (set `self.GrabbedActor` _array_element))
          (set `self.NearestOverlap` _returnvalue)
          (message `/Game/VirtualRealityBP/Blueprints/PickupActorInterface.Pickup` _output_get (`self.Sphere`))
          (`KismetSystemLibrary.PrintString` (`KismetSystemLibrary.GetDisplayName` _output_get))))))
  (:`Released`
    (goto _label)))

(fn `FireRay`
  (bind _rootcomponent (`Actor.RootComponent` (`GameplayStatics.GetPlayerCameraManager` 0)))
  (bind _returnvalue (`SceneComponent.K2_GetComponentLocation` _rootcomponent))
  (bind (_outhit _returnvalue_2) (`KismetSystemLibrary.LineTraceSingleForObjects` _returnvalue (+ _returnvalue (* (`KismetMathLibrary.GetForwardVector` (`SceneComponent.K2_GetComponentRotation` _rootcomponent)) 1500.0)) (`|MakeArray` "ObjectTypeQuery2" :!type "EObjectTypeQuery Enum")))
  (if _returnvalue_2
    (message `/Game/VRBurnLab/Core/Character/RayActorInterface.RayInteract` (`.HitActor` (`GameplayStatics.BreakHitResult` _outhit)))))

(fn `UserConstructionScript`)