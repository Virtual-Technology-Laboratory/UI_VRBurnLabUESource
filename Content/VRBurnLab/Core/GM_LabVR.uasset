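; VR burn lab game mode that gates the assembly steps by revealing ghost actors in order.
; BeginPlay hides and disables collision on all ghost table jacks, boards, saplings and needles.
; Tick polls nested progress checks (Bricks, Jacks, Board, Sapling), each using a DoOnce to reveal the next ghost set with collision.
; The final Needles check triggers nothing, and the progress variables are not set in this graph.
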(event `self.ReceiveBeginPlay`
  (`|ExecutionSequence`
    (:`then_0`
      (bind _outactors (`GameplayStatics.GetAllActorsOfClass` "/Game/VRBurnLab/Placeables/Ghosts/BP_GhostTableJack.BP_GhostTableJack_C"))
      (for _array_element _outactors
        (`self.SetActorHiddenInGame` _array_element true)
        (`self.SetActorEnableCollision` _array_element false)))
    (:`then_1`
      (bind _outactors_2 (`GameplayStatics.GetAllActorsOfClass` "/Game/VRBurnLab/Placeables/Ghosts/BP_GhostBoard.BP_GhostBoard_C"))
      (for _array_element_2 _outactors_2
        (`self.SetActorHiddenInGame` _array_element_2 true)
        (`self.SetActorEnableCollision` _array_element_2 false)))
    (:`then_2`
      (bind _outactors_3 (`GameplayStatics.GetAllActorsOfClass` "/Game/VRBurnLab/Placeables/Ghosts/BP_GhostSapling.BP_GhostSapling_C"))
      (for _array_element_3 _outactors_3
        (`self.SetActorHiddenInGame` _array_element_3 true)
        (`self.SetActorEnableCollision` _array_element_3 false)))
    (:`then_3`
      (bind _outactors_4 (`GameplayStatics.GetAllActorsOfClass` "/Game/VRBurnLab/Placeables/Ghosts/BP_GhostNeedles.BP_GhostNeedles_C"))
      (for _array_element_4 _outactors_4
        (`self.SetActorHiddenInGame` _array_element_4 true)
        (`self.SetActorEnableCollision` _array_element_4 false)))))

(event `self.ReceiveTick`
  (params (DeltaSeconds :type "Float (single-precision)"))
  (if (>= (`self.Bricks`) 4)
    (`|ExecutionSequence`
      (:`then_0`
        (`/Engine/EditorBlueprintResources/StandardMacros.DoOnce` false
          (:`Completed`
            (`KismetSystemLibrary.PrintString` "JACKS!!!!!")
            (for _array_element (stale `self.ReceiveBeginPlay` _outactors)
              (`self.SetActorHiddenInGame` _array_element false)
              (`self.SetActorEnableCollision` _array_element true)))))
      (:`then_1`
        (if (>= (`self.Jacks`) 3)
          (`|ExecutionSequence`
            (:`then_0`
              (`/Engine/EditorBlueprintResources/StandardMacros.DoOnce` false
                (:`Completed`
                  (for _array_element_2 (stale `self.ReceiveBeginPlay` _outactors_2)
                    (`self.SetActorHiddenInGame` _array_element_2 false)
                    (`self.SetActorEnableCollision` _array_element_2 true)))))
            (:`then_1`
              (if (`self.Board`)
                (`|ExecutionSequence`
                  (:`then_0`
                    (`/Engine/EditorBlueprintResources/StandardMacros.DoOnce` false
                      (:`Completed`
                        (for _array_element_3 (stale `self.ReceiveBeginPlay` _outactors_3)
                          (`self.SetActorHiddenInGame` _array_element_3 false)
                          (`self.SetActorEnableCollision` _array_element_3 true)))))
                  (:`then_1`
                    (if (`self.Sapling`)
                      (`|ExecutionSequence`
                        (:`then_0`
                          (`/Engine/EditorBlueprintResources/StandardMacros.DoOnce` false
                            (:`Completed`
                              (for _array_element_4 (stale `self.ReceiveBeginPlay` _outactors_4)
                                (`self.SetActorHiddenInGame` _array_element_4 false)
                                (`self.SetActorEnableCollision` _array_element_4 true)))))
                        (:`then_1`
                          (if (`self.Needles`)
                            (`/Engine/EditorBlueprintResources/StandardMacros.DoOnce` false)))))))))))))))

(fn `UserConstructionScript`)