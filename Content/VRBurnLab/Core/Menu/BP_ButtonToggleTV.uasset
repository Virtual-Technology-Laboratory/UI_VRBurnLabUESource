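; VR menu button that, despite its ToggleTV name, opens the VRBurnLab_v03 level.
; BeginPlay caches the right controller from the first MotionControllerPawn.
; Any overlap recolors the text, and both begin and end events set IsOverlaped by comparing the actor to that controller, so leaving does not clear it.
; Releasing R_Trigger while flagged loads the level through a resettable DoOnce and prints a debug string.
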(event `self.ReceiveBeginPlay`
  (bind _outactors (`GameplayStatics.GetAllActorsOfClass` "/Game/VirtualRealityBP/Blueprints/MotionControllerPawn.MotionControllerPawn_C"))
  (set `self.Right Controller` (`/Game/VirtualRealityBP/Blueprints/MotionControllerPawn.RightController` (`|GetArrayItem` _outactors))))

(event `self.ReceiveActorBeginOverlap`
  (params (OtherActor :type "Actor Object Reference"))
  (set `self.IsOverlaped` (== OtherActor (`self.Right Controller`)))
  (`TextRenderComponent.SetTextRenderColor` (`self.text`) (`KismetMathLibrary.Conv_LinearColorToColor` (`KismetMathLibrary.MakeColor` 0.0 0.0 1.0))))

(event `self.ReceiveActorEndOverlap`
  (params (OtherActor :type "Actor Object Reference"))
  (set `self.IsOverlaped` (== OtherActor (`self.Right Controller`)))
  (`TextRenderComponent.SetTextRenderColor` (`self.text`) (`KismetMathLibrary.Conv_LinearColorToColor` (`KismetMathLibrary.MakeColor` 0.0))))

(event `InputAction|R_Trigger`
  (params (Key :type "Key Structure"))
  (:`Released`
    (if (`self.IsOverlaped`)
      (`|DoOnceMultiInput` :!label _label
        (:`A Out`
          (`GameplayStatics.OpenLevelBySoftObjectPtr` "/Game/VRBurnLab/Maps/VRBurnLab_v03.VRBurnLab_v03" false)
          (`KismetSystemLibrary.PrintString` "ButtonPress")
          (goto _label :!via `Reset In`))))))

(fn `UserConstructionScript`
  (`parent.UserConstructionScript`))