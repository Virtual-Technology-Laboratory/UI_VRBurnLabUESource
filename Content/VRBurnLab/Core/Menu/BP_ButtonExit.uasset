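; VR menu exit button that opens the BirdHouse_v01 level when it receives a RayInteract event.
; A DoOnce gate resets after a short delay to debounce repeated presses.
; Any actor overlap tints the text blue and overlap end restores the default color.
; Both overlap events also set IsOverlaped by comparing against the pawn's right controller, but nothing here reads that flag.
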(event `self.ReceiveBeginPlay`
  (bind _outactors (`GameplayStatics.GetAllActorsOfClass` "/Game/VirtualRealityBP/Blueprints/MotionControllerPawn.MotionControllerPawn_C"))
  (set `self.Right Controller` (`/Game/VirtualRealityBP/Blueprints/MotionControllerPawn.RightController` (`|GetArrayItem` _outactors))))

(event `self.ReceiveActorBeginOverlap`
  (params (OtherActor :type "Actor Object Reference"))
  (set `self.IsOverlaped` (== OtherActor (`self.Right Controller`)))
  (`TextRenderComponent.SetTextRenderColor` (`self.text`) (`KismetMathLibrary.Conv_LinearColorToColor` (`KismetMathLibrary.MakeColor` 0.0 0.0 1.0))))

(event `self.ReceiveActorEndOverlap`
  (params (OtherActor :type "Actor Object Reference"))
  (set `self.IsOverlaped` (== OtherActor (`self.Right Controller`)))
  (`TextRenderComponent.SetTextRenderColor` (`self.text`) (`KismetMathLibrary.Conv_LinearColorToColor` (`KismetMathLibrary.MakeColor` 0.0))))

(event `/Game/VRBurnLab/Core/Character/RayActorInterface.RayInteract`
  (`|DoOnceMultiInput` :!label _label
    (:`A Out`
      (`GameplayStatics.OpenLevelBySoftObjectPtr` "/Game/VRBurnLab/Maps/BirdHouse_v01.BirdHouse_v01" false)
      (`KismetSystemLibrary.Delay` 0.2)
      (goto _label :!via `Reset In`))))

(fn `UserConstructionScript`
  (`parent.UserConstructionScript`))