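; BP_UIEFPoster is a VR menu poster that opens the UIEF site level when it receives RayInteract.
; RayInteract passes through a DoOnce MultiInput gate, opens the level by object reference, prints a debug string, then resets the gate.
; Older logic for right-controller overlap and trigger press remains in the graph but is disconnected, leaving BeginPlay and both overlap events empty.
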(event `self.ReceiveBeginPlay`)

(event `self.ReceiveActorBeginOverlap`
  (params (OtherActor :type "Actor Object Reference")))

(event `self.ReceiveActorEndOverlap`
  (params (OtherActor :type "Actor Object Reference")))

(event `InputAction|R_Trigger`
  (params (Key :type "Key Structure")))

(event `/Game/VRBurnLab/Core/Character/RayActorInterface.RayInteract`
  (`|DoOnceMultiInput` :!label _label
    (:`A Out`
      (`GameplayStatics.OpenLevelBySoftObjectPtr` "/Game/VRBurnLab/Maps/UIEFSite.UIEFSite" false)
      (`KismetSystemLibrary.PrintString` "Should be opening level..")
      (goto _label :!via `Reset In`))))

(fn `UserConstructionScript`
  (`parent.UserConstructionScript`))