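; BP_MenuBox is a VR menu trigger volume that shows the right motion controller's pointer and pointer ball while that controller overlaps it.
; On BeginPlay it caches the RightController from the first MotionControllerPawn found.
; If the player pawn's object name matches BP_FPS_C_0, it sets a Testing flag and disables its collision instead.
; Begin and end overlap events toggle the pointer visibility for that controller only.
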(event `self.ReceiveBeginPlay`
  (bind _output_get (set `self.Testing` (`KismetStringLibrary.EqualEqual_StrStr` (`KismetSystemLibrary.GetObjectName` (`GameplayStatics.GetPlayerPawn` 0)) "BP_FPS_C_0")))
  (if _output_get
    (`PrimitiveComponent.SetCollisionEnabled` (`self.CollisionComponent`) "NoCollision")
    (else
      (bind _outactors (`GameplayStatics.GetAllActorsOfClass` "/Game/VirtualRealityBP/Blueprints/MotionControllerPawn.MotionControllerPawn_C"))
      (set `self.Right Controller` (`/Game/VirtualRealityBP/Blueprints/MotionControllerPawn.RightController` (`|GetArrayItem` _outactors))))))

(event `self.ReceiveActorBeginOverlap`
  (params (OtherActor :type "Actor Object Reference"))
  (bind _right_controller (`self.Right Controller`))
  (if (== OtherActor _right_controller)
    (`SceneComponent.SetVisibility` (`/Game/VirtualRealityBP/Blueprints/BP_MotionController.pointer` _right_controller) true false)
    (`SceneComponent.SetVisibility` (`/Game/VirtualRealityBP/Blueprints/BP_MotionController.pointer_ball` _right_controller) true false)))

(event `self.ReceiveActorEndOverlap`
  (params (OtherActor :type "Actor Object Reference"))
  (bind _right_controller (`self.Right Controller`))
  (if (== OtherActor _right_controller)
    (`SceneComponent.SetVisibility` (`/Game/VirtualRealityBP/Blueprints/BP_MotionController.pointer` _right_controller) false false)
    (`SceneComponent.SetVisibility` (`/Game/VirtualRealityBP/Blueprints/BP_MotionController.pointer_ball` _right_controller) false false)))

(fn `UserConstructionScript`)